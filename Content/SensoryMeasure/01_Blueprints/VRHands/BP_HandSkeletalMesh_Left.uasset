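; Left VR hand Blueprint for the SensoryMeasure project, carrying a holographic debug readout.
; InitializeDebugComponents caches the WBP_DebugText widget and hides the debug components, but nothing in this file calls it.
; Disconnected logic would toggle the readout on a time-gated left-index-finger overlap with a Niagara burst, and write name/value text to the widget.
; All event entry points are empty, so none of that logic runs.
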(event OnComponentBeginOverlap(DebugAreaCollider)
  (params (OverlappedComponent :type Primitive%20Component%20Object%20Reference) (OtherActor :type Actor%20Object%20Reference) (OtherComp :type Primitive%20Component%20Object%20Reference) (OtherBodyIndex :type Integer) (bFromSweep :type Boolean) (SweepResult :type Hit%20Result%20Structure%20%28by%20ref%29))
  ;[0 0.4339 1] Active Debug Components
)

(event EventBeginPlay)

(event Collision|EventActorBeginOverlap
  (params (OtherActor :type Actor%20Object%20Reference)))

(event EventUpdateDebugText
  (params (VariableName :type String) (VariableValue :type String))
  ;[1 1 1] Debug Visualization
)

(event EventToggleDebugVisualization
  ;[1 1 1] Debug Visualization
)

(event EventTick
  (params (DeltaSeconds :type Float%20%28single-precision%29)))

(fn ConstructionScript)

(fn InitializeDebugComponents
  (bind _widget (Variables|Default|GetWidget))
  (Variables|Default|SetDebugWidgetComponent _widget)
  (bind _aswbp_debug_text (Utilities|Casting|CastToWBP_DebugText (UserInterface|GetWidget _widget)))
  (Variables|Default|SetDebug%20Text%20Widget _aswbp_debug_text)
  (Development|SetHiddeninGame (Variables|Default|GetDebugComponents) true true))