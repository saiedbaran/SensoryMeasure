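; VR game mode for the SensoryMeasure study that handles Lab Streaming Layer (LSL) event messaging.
; On BeginPlay it applies the study data's VR pixel density by console command, binds the LSL inlet and caches the NPCP game instance.
; Incoming inlet strings are printed on screen for debugging.
; OnLSLEvent pushes event strings to the LSL outlet and briefly prints them with game time.
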(event Custom|OnStreamUpdatedString_Event
  (params (StringArray :type Array%20of%20Strings) (DeltaSeconds :type Float%20%28single-precision%29))
  (Development|PrintString (Utilities|String|Append (Utilities|Array|Get(acopy) StringArray) ": " (Utilities|String|ToString(Float) DeltaSeconds)) true true "(R=0.326711,G=0.000000,B=1.000000,A=1.000000)" 2e+01))

(event EventBeginPlay
  (Development|ExecuteConsoleCommand (Utilities|String|Append "vr.PixelDensity " (Utilities|String|ToString(Float) (Variables|/Script/VRCharacter.StudyData|GetPixelDensity (Variables|Default|GetStudyData)))) 0)
  (EventDispatchers|AssignOnStreamUpdatedString (Variables|Default|GetLSLInlet) (delegate Custom|OnStreamUpdatedString_Event))
  (bind _asbp_game_instance_npcp (Utilities|Casting|CastToBP_GameInstance_NPCP (Game|GetGameInstance))))

(event EventTick
  (params (DeltaSeconds :type Float%20%28single-precision%29)))

(event EventOnLSLEvent
  (params (EventData :type String))
  (Class|LSLOutletComponent|PushSampleString (Variables|Default|GetLSLOutlet) (Utilities|Array|MakeArray EventData))
  (Development|PrintString (Utilities|String|Append EventData ": " (Utilities|String|ToString(Float) (Utilities|Time|GetTimeSeconds))) true true "(R=0.000000,G=0.660000,B=1.000000,A=1.000000)" 0.1))

(fn ConstructionScript)